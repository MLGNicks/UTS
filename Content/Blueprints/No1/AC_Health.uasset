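; AC_Health is a health component that tracks hit points and a death state for its owning actor.
; On BeginPlay it fills HP to MaxHP and binds to the owner's OnTakeAnyDamage event.
; Incoming damage is negated and passed to AdjustDamage, which adds it to HP clamped between zero and MaxHP.
; When HP reaches zero it calls Death, which only sets the Dead flag.
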(event Custom|Damaged
  (params (DamagedActor :type Actor%20Object%20Reference) (Damage :type Float%20%28single-precision%29) (DamageType :type Damage%20Type%20Object%20Reference) (InstigatedBy :type Controller%20Object%20Reference) (DamageCauser :type Actor%20Object%20Reference))
  (CallFunction|AdjustDamage (* Damage -1.0)))

(event Custom|AdjustDamage
  (params (AddHP :type Float%20%28double-precision%29))
  (Variables|Default|SetHP (Math|Float|Clamp(Float) (+ (Variables|Default|GetHP) AddHP) 0.0 (Variables|Default|GetMaxHP)))
  (if (<= (Variables|Default|GetHP) 0.0)
    (CallFunction|Death)))

(event Custom|Death
  (Variables|Default|SetDead true))

(event EventBeginPlay
  (Variables|Default|SetHP (Variables|Default|GetMaxHP))
  (bind _output_get (Variables|Default|SetOwner (Components|GetOwner)))
  (EventDispatchers|BindEventtoOnTakeAnyDamage _output_get (delegate Custom|Damaged)))